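; OLD_DungeonNode is a world map node Blueprint for a dungeon, with an OLD prefix in its name, that highlights under the cursor.
; The construction script applies the Mesh and Material variables to its NodeMesh component.
; Cursor-over events swap the slot 0 material to HoverMaterial and restore Material when the cursor leaves.
; It contains no selection or travel logic.
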(event `self.ReceiveActorBeginCursorOver`
  (`PrimitiveComponent.SetMaterial` 0 (`self.HoverMaterial`)))

(event `self.ReceiveActorEndCursorOver`
  (`PrimitiveComponent.SetMaterial` 0 (`self.Material`)))

(fn `UserConstructionScript`
  (bind _nodemesh (`self.NodeMesh`))
  (`PrimitiveComponent.SetMaterial` _nodemesh 0 (`self.Material`))
  (`StaticMeshComponent.SetStaticMesh` _nodemesh (`self.Mesh`)))