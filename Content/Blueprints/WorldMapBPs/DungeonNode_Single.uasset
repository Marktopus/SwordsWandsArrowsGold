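; World map dungeon node that grows a branching path of child nodes; clicking an unexplored one saves the party and opens the TEST level.
; RevealNode records the chosen sibling index on the root and marks the node and its siblings explored.
; MakeNode recursively extends the tree per reveal, spawning one to three evenly spaced nodes with SplinePath links, using a per-height count array.
; Children inherit that array and root, and share a sibling list.
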(event Custom|RevealNode
  ;[1 1 1] On Clicked
  ;;[1 1 1] Make Nodes
  (if (not (Variables|Default|GetHasExplored))
    (bind _succes (CallFunction|MakeNode (Utilities|Array|Get(acopy) (Variables|Default|GetNumOfSiblingsPerHeight) (+ (Variables|Default|GetHeight) 1))))
    (Utilities|Array|Add (Variables|DungeonNode_Single_C|GetRevealedIndexPerHeight (Variables|Default|GetRoot)) (Variables|Default|GetSiblingIndex))
    (Variables|Default|SetHasExplored true)
    (for _array_element (Variables|Default|GetSiblingNodes)
      (Variables|DungeonNode_Single_C|SetHasExplored _array_element true))))

(event EventActorOnClicked
  ;[1 1 1] On Clicked
  (if (not (Variables|Default|GetHasExplored))
    (bind _asworld_map_mode (Utilities|Casting|CastToWorldMapMode (Game|GetGameMode)))
    (Default|SaveParty _asworld_map_mode (Variables|Default|GetSiblingIndex))
    (Game|LoadStreamLevel(byName) "TEST" false)
    (Game|OpenLevel(byName) "TEST")))

(fn ConstructionScript
  (if (Variables|Node|GetIsRoot)
    (Variables|Default|SetRoot self)))

(fn MakeNode
  (params (NumOfNodes :type Integer))
  (bind _returnvalue (Transformation|GetActorLocation))
  (bind _returnvalue_2 (- NumOfNodes 1))
  (bind _nextnodespacing (Variables|Default|GetNextNodeSpacing))
  (bind _childnodes (Variables|Default|GetChildNodes))
  (bind _nextnodedistance (Variables|Default|GetNextNodeDistance))
  (bind _returnvalue_3 (* _nextnodedistance -1.0))
  (bind _returnvalue_4 (Math|Vector|MakeVector _returnvalue_3 0.0 0.0))
  (bind _returnvalue_5 (+ _returnvalue _returnvalue_4))
  (Variables|Default|SetHasExplored true)
  (for _array_element (Variables|Default|GetSiblingNodes)
    (Variables|DungeonNode_Single_C|SetHasExplored _array_element true))
  (LocalVariables|SetFirstNodePos (+ (Transformation|GetActorLocation) (Math|Vector|MakeVector (* (Variables|Default|GetNextNodeDistance) -1.0) 0.0 0.0)))
  (switch int NumOfNodes
    (:0
      ;[1 1 1] Singe Path
      (LocalVariables|SetIsSuccessful false))
    (:1
      (bind _returnvalue_6 (Game|SpawnActorfromClass "/Game/Blueprints/WorldMapBPs/SplinePath.SplinePath_C" (Transformation|GetActorTransform) false 0))
      (Class|SplineComponent|SetWorldLocationatSplinePoint (Variables|/Game/Blueprints/WorldMapBPs/SplinePath.SplinePath_C|GetSpline _returnvalue_6) 1 _returnvalue_5)
      (Default|MakePath _returnvalue_6 1e+02)
      (bind _returnvalue_7 (Game|SpawnActorfromClass "DungeonNode_Single_C" (Math|Transform|MakeTransform _returnvalue_5) true 0))
      (Variables|DungeonNode_Single_C|SetNumOfSiblingsPerHeight _returnvalue_7 (Variables|Default|GetNumOfSiblingsPerHeight))
      (Variables|DungeonNode_Single_C|SetHeight _returnvalue_7 (+ (Variables|Default|GetHeight) 1))
      (Variables|DungeonNode_Single_C|SetSiblingIndex _returnvalue_7 1)
      (Utilities|Array|Add (Variables|Default|GetChildNodes) _returnvalue_7)
      (Variables|DungeonNode_Single_C|SetRoot _returnvalue_7 (Variables|Default|GetRoot))
      (for _array_element_2 _childnodes :!label _label
        (Variables|DungeonNode_Single_C|SetSiblingNodes _array_element_2 _childnodes)
        (LocalVariables|SetIsSuccessful true)
        (return (LocalVariables|GetIsSuccessful))))
    (:2
      ;[1 1 1] Multiple Paths
      (for _index (range 0 _returnvalue_2) :!label _label_2
        (bind _returnvalue_8 (Game|SpawnActorfromClass "/Game/Blueprints/WorldMapBPs/SplinePath.SplinePath_C" (Transformation|GetActorTransform) false 0))
        (Class|SplineComponent|SetWorldLocationatSplinePoint (Variables|/Game/Blueprints/WorldMapBPs/SplinePath.SplinePath_C|GetSpline _returnvalue_8) 1 (- (+ (LocalVariables|GetFirstNodePos) (Math|Vector|MakeVector 0.0 (* _index (* _nextnodespacing 2.0)) 0.0)) (Math|Vector|MakeVector 0.0 (* _returnvalue_2 _nextnodespacing) 0.0)))
        (Default|MakePath _returnvalue_8 1e+02)
        (bind _returnvalue_9 (Game|SpawnActorfromClass "DungeonNode_Single_C" (Math|Transform|MakeTransform (- (+ (LocalVariables|GetFirstNodePos) (Math|Vector|MakeVector 0.0 (* _index (* _nextnodespacing 2.0)) 0.0)) (Math|Vector|MakeVector 0.0 (* _returnvalue_2 _nextnodespacing) 0.0))) true 0))
        (Utilities|Array|Add (Variables|Default|GetChildNodes) _returnvalue_9)
        (Variables|DungeonNode_Single_C|SetNumOfSiblingsPerHeight _returnvalue_9 (Variables|Default|GetNumOfSiblingsPerHeight))
        (Variables|DungeonNode_Single_C|SetHeight _returnvalue_9 (+ (Variables|Default|GetHeight) 1))
        (Variables|DungeonNode_Single_C|SetSiblingIndex _returnvalue_9 (+ _index 1))
        (Variables|DungeonNode_Single_C|SetRoot _returnvalue_9 (Variables|Default|GetRoot)))
      (goto _label))
    (:3
      (goto _label_2))))

(fn GetChildNodes
  (return (Variables|Default|GetChildNodes)))