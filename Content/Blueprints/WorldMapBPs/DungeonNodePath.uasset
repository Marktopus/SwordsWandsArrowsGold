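; World map dungeon path actor that places OLD_DungeonNode child actors and spline mesh lines at even spacing along a spline.
; Construction builds the path when Preview is set, while RevealNextNode adds one node and segment per call.
; BeginPlay jitters interior spline points, and the main path links other DungeonNodePath actors to its nodes as left or right branches by parent or exit index.
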(event EventBeginPlay
  (bind _spline (Variables|Default|GetSpline))
  (bind _returnvalue (Class|SplineComponent|GetNumSplinePoints _spline))
  (bind _returnvalue_2 (- _returnvalue 1))
  ;[1 1 1] RandomPos
  (Utilities|FlowControl|Sequence
    (:then_0
      (for _index (range 0 _returnvalue_2)
        (if (!= _index 0)
          (if (!= _index _returnvalue_2)
            (Class|SplineComponent|SetWorldLocationatSplinePoint _spline _index (Math|Vector|MakeVector (+ (.X (Math|Vector|BreakVector (Class|SplineComponent|GetWorldLocationatSplinePoint _spline _index))) (Math|Random|RandomFloatinRange -6e+01 -3e+01)) (+ (.Y (Math|Vector|BreakVector (Class|SplineComponent|GetWorldLocationatSplinePoint _spline _index))) (Math|Random|RandomFloatinRange -6e+01 6e+01)) (.Z (Math|Vector|BreakVector (Class|SplineComponent|GetWorldLocationatSplinePoint _spline _index)))))))))
    (:then_1
      (if (Variables|PathGen|GetMainPath)
        (for (_array_element _array_index) (Variables|Default|GetNodes)
          (bind _outactors (Actor|GetAllActorsOfClass "DungeonNodePath_C"))
          (for _array_element_2 _outactors
            (if (!= _array_element_2 self)
              (if (or (== (Variables|DungeonNodePath_C|GetParentNodeIndex _array_element_2) _array_index) (== (Variables|DungeonNodePath_C|GetExitNodeIndex _array_element_2) _array_index))
                (Utilities|FlowControl|Sequence
                  (:then_0
                    (if (Variables|DungeonNodePath_C|GetIsLeftOfParent _array_element_2)
                      (Variables|/Game/Blueprints/WorldMapBPs/OLD_DungeonNode.OLD_DungeonNode_C|SetChildNodeToLeftPath _array_element _array_element_2)
                      (else
                        (Variables|/Game/Blueprints/WorldMapBPs/OLD_DungeonNode.OLD_DungeonNode_C|SetChildNodeToRightPath _array_element _array_element_2))))
                  (:then_1
                    (if (Variables|DungeonNodePath_C|GetIsLeftOfParent _array_element_2)
                      _)))))))))))

(fn ConstructionScript
  (bind _maximumnodes (Variables|PathGen|GetMaximumNodes))
  (bind _tangentscale (Variables|PathGen|GetTangentScale))
  (bind _spline (Variables|Default|GetSpline))
  (bind _spacing (Variables|PathGen|GetSpacing))
  (bind _spacing_2 (Variables|PathGen|GetSpacing))
  (bind _spline_2 (Variables|Default|GetSpline))
  (bind _returnvalue (- _maximumnodes 1))
  (Utilities|Array|Clear (Variables|Default|GetNodes))
  (if (Variables|PathGen|GetPreview)
    (Utilities|FlowControl|Sequence
      (:then_0
        ;[1 1 1] Generate Node Based On Length
        (if (Variables|PathGen|GetHasStartingNode)
          (LocalVariables|SetNodeStartingIndex 0)
          (else
            (LocalVariables|SetNodeStartingIndex 1)))
        (for _index (range (LocalVariables|GetNodeStartingIndex) (.ReturnValue (Math|Float|Division(WholeandRemainder) (Spline|GetSplineLength _spline_2) _spacing)))
          (if (< _index (Variables|PathGen|GetMaximumNodes))
            (CallFunction|AddNode (Math|Transform|MakeTransform (Class|SplineComponent|GetWorldLocationatDistanceAlongSpline _spline_2 (* _index _spacing)))))))
      (:then_1
        ;[1 1 1] Generate Path Based On Length
        (for _index_2 (range 0 (.ReturnValue (Math|Float|Division(WholeandRemainder) (Spline|GetSplineLength _spline) _spacing_2)))
          (if (< _index_2 _returnvalue)
            (bind _returnvalue_2 (AddComponent|AddSplineMeshComponent true :!label _label))
            (SplineMesh|SetStartandEnd _returnvalue_2 (Class|SplineComponent|GetWorldLocationatDistanceAlongSpline _spline (* _index_2 _spacing_2)) (* (Class|SplineComponent|GetWorldDirectionatDistanceAlongSpline _spline (* _index_2 _spacing_2)) _tangentscale) (Class|SplineComponent|GetWorldLocationatDistanceAlongSpline _spline (+ (* _index_2 _spacing_2) _spacing_2)) (* (Class|SplineComponent|GetWorldDirectionatDistanceAlongSpline _spline (+ (* _index_2 _spacing_2) _spacing_2)) _tangentscale) :!class /Script/Engine.SplineMeshComponent)
            (Components|StaticMesh|SetStaticMesh _returnvalue_2 (Variables|PathGen|GetLineMesh))
            (Rendering|Material|SetMaterial _returnvalue_2 0 (Variables|PathGen|GetLineMaterial))
            (elif (Variables|PathGen|GetHasEndingNode)
              (if (== _index_2 _returnvalue)
                (goto _label))))))
      (:then_2
        (Variables|PathGen|SetCurrentlyRevealedNodes (+ (Variables|PathGen|GetCurrentlyRevealedNodes) 1))))))

(fn AddNode
  (params (Transform :type Transform))
  (bind _nodes (Variables|Default|GetNodes))
  (bind _returnvalue (Utilities|Array|Length _nodes))
  (bind _returnvalue_2 (AddComponent|AddChildActorComponent true Transform))
  (bind _asold_dungeon_node (Utilities|Casting|CastToOLD_DungeonNode (Variables|/Script/Engine.ChildActorComponent|GetChildActor _returnvalue_2)))
  (if (Variables|PathGen|GetMainPath)
    (if (< _returnvalue (- (Variables|PathGen|GetMaximumNodes) 1))
      (if (> _returnvalue 0)
        (Rendering|Material|SetMaterial _asold_dungeon_node 0 (Variables|PathGen|GetSplineMaterial) :!label _label)
        (Components|StaticMesh|SetStaticMesh _asold_dungeon_node (Variables|PathGen|GetSplineMesh))
        (else
          (Rendering|Material|SetMaterial _asold_dungeon_node 0 (Variables|Tips|GetExitMaterial))
          (Components|StaticMesh|SetStaticMesh _asold_dungeon_node (Variables|Tips|GetEntranceMesh))))
      (else
        (Rendering|Material|SetMaterial _asold_dungeon_node 0 (Variables|Tips|GetExitMaterial))
        (Components|StaticMesh|SetStaticMesh _asold_dungeon_node (Variables|Tips|GetExitMesh))))
    (else
      (goto _label)))
  (bind _returnvalue_3 (Utilities|Array|Add (Variables|Default|GetNodes) _asold_dungeon_node))
  (Variables|/Game/Blueprints/WorldMapBPs/OLD_DungeonNode.OLD_DungeonNode_C|SetIndex _asold_dungeon_node _returnvalue_3)
  (Variables|/Game/Blueprints/WorldMapBPs/OLD_DungeonNode.OLD_DungeonNode_C|SetMyPath _asold_dungeon_node self))

(fn RevealNextNode
  (bind _tangentscale (Variables|PathGen|GetTangentScale))
  (bind _spline (Variables|Default|GetSpline))
  (bind _spacing (Variables|PathGen|GetSpacing))
  (if (< (Variables|PathGen|GetCurrentlyRevealedNodes) (Variables|PathGen|GetMaximumNodes))
    (Utilities|FlowControl|Sequence
      (:then_0
        ;[1 1 1] Generate Node Based On Length
        (LocalVariables|SetRevealedNodesMod 0)
        (if (Variables|PathGen|GetHasStartingNode)
          _
          (else
            (LocalVariables|SetRevealedNodesMod 1)))
        (CallFunction|AddNode (Math|Transform|MakeTransform (Class|SplineComponent|GetWorldLocationatDistanceAlongSpline (Variables|Default|GetSpline) (* (+ (Variables|PathGen|GetCurrentlyRevealedNodes) (LocalVariables|GetRevealedNodesMod)) (Variables|PathGen|GetSpacing))) "0, 0, 0" "1,1,1.000000")))
      (:then_1
        ;[1 1 1] Generate Path Based On Length
        (if (> (Variables|PathGen|GetCurrentlyRevealedNodes) 0)
          (bind _returnvalue (AddComponent|AddSplineMeshComponent true :!label _label))
          (SplineMesh|SetStartandEnd _returnvalue (Class|SplineComponent|GetWorldLocationatDistanceAlongSpline _spline (* (+ (- (Variables|PathGen|GetCurrentlyRevealedNodes) 1) (LocalVariables|GetRevealedNodesMod)) _spacing)) (* (Class|SplineComponent|GetWorldDirectionatDistanceAlongSpline _spline (* (+ (- (Variables|PathGen|GetCurrentlyRevealedNodes) 1) (LocalVariables|GetRevealedNodesMod)) _spacing)) _tangentscale) (Class|SplineComponent|GetWorldLocationatDistanceAlongSpline _spline (+ (* (+ (- (Variables|PathGen|GetCurrentlyRevealedNodes) 1) (LocalVariables|GetRevealedNodesMod)) _spacing) _spacing)) (* (Class|SplineComponent|GetWorldDirectionatDistanceAlongSpline _spline (+ (* (+ (- (Variables|PathGen|GetCurrentlyRevealedNodes) 1) (LocalVariables|GetRevealedNodesMod)) _spacing) _spacing)) _tangentscale) :!class /Script/Engine.SplineMeshComponent)
          (Components|StaticMesh|SetStaticMesh _returnvalue (Variables|PathGen|GetLineMesh))
          (Rendering|Material|SetMaterial _returnvalue 0 (Variables|PathGen|GetLineMaterial))
          (elif (not (Variables|PathGen|GetHasStartingNode))
            (goto _label))))
      (:then_2
        (Variables|PathGen|SetCurrentlyRevealedNodes (+ (Variables|PathGen|GetCurrentlyRevealedNodes) 1))))))

(fn GetLeftPathOfNode
  (params (Index :type Integer))
  (return (Variables|/Game/Blueprints/WorldMapBPs/OLD_DungeonNode.OLD_DungeonNode_C|GetChildNodeToLeftPath (Utilities|Array|Get(acopy) (Variables|Default|GetNodes) Index))))

(fn GetRightPathOfNode
  (params (Index :type Integer))
  (return (Variables|/Game/Blueprints/WorldMapBPs/OLD_DungeonNode.OLD_DungeonNode_C|GetChildNodeToRightPath (Utilities|Array|Get(acopy) (Variables|Default|GetNodes) Index))))