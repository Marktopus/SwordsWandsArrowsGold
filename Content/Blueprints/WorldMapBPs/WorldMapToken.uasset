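; World map token pawn that travels node to node along branching DungeonNodePath actors, starting on the one flagged MainPath.
; Next and previous step along the current path, crossing to its exit or parent path at the ends.
; Left and right query only MainPath for side branches, entering at either end.
; Each move uses AIMoveTo behind a Moving lock, which clears on success but not on failure.
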(event `self.ReceiveBeginPlay`
  (bind _mainpath (`self.MainPath`))
  (bind _outactors (`GameplayStatics.GetAllActorsOfClass` "/Game/Blueprints/WorldMapBPs/DungeonNodePath.DungeonNodePath_C"))
  (for _array_element _outactors
    (if (`/Game/Blueprints/WorldMapBPs/DungeonNodePath.MainPath` _array_element)
      (set `self.MainPath` _array_element)
      (set `self.CurrentNode` (`KismetArrayLibrary.Array_Get` (`/Game/Blueprints/WorldMapBPs/DungeonNodePath.Nodes` _mainpath) (`self.CurrentNodeIndex`)))
      (set `self.CurrenPath` _mainpath))))

(event `MoveToNode`
  (bind _targetnode (`self.TargetNode`))
  (`|AIMoveTo` self (`SceneComponent.K2_GetComponentLocation` (`self.TargetNode`)) null 0.005
    (:`then`
      (set `self.Moving` true))
    (:`OnSuccess`
      (`KismetSystemLibrary.PrintString` "yes")
      (set `self.CurrentNode` _targetnode)
      (set `self.Moving` false)
      (set `self.CurrenPath` (`/Game/Blueprints/WorldMapBPs/OLD_DungeonNode.MyPath` _targetnode))
      (set `self.CurrentNodeIndex` (`/Game/Blueprints/WorldMapBPs/OLD_DungeonNode.Index` _targetnode)))
    (:`OnFail`
      (`KismetSystemLibrary.PrintString` "Hello"))))

(fn `MoveToLeftNode`
  (bind _currentnodeindex (`self.CurrentNodeIndex`))
  (if (`self.Moving`)
    _
    (elif true
      (bind _childpath (`/Game/Blueprints/WorldMapBPs/DungeonNodePath.GetLeftPathOfNode` (`self.MainPath`) _currentnodeindex))
      (`/Engine/EditorBlueprintResources/StandardMacros.IsValid` _childpath
        (:`Is Valid`
          (if (== (`/Game/Blueprints/WorldMapBPs/DungeonNodePath.ExitNodeIndex` _childpath) _currentnodeindex)
            (bind _nodes (`/Game/Blueprints/WorldMapBPs/DungeonNodePath.Nodes` _childpath))
            (bind _returnvalue (- (`KismetArrayLibrary.Array_Length` (`/Game/Blueprints/WorldMapBPs/DungeonNodePath.Nodes` _childpath)) 1))
            (`self.UpdateNodeInfo` (`KismetArrayLibrary.Array_Get` _nodes _returnvalue) _returnvalue)
            (`self.MoveToNode` :!label _label)
            (elif (== (`/Game/Blueprints/WorldMapBPs/DungeonNodePath.ParentNodeIndex` _childpath) _currentnodeindex)
              (`self.UpdateNodeInfo` (`KismetArrayLibrary.Array_Get` _nodes))
              (goto _label))))))))

(fn `MoveToNextNode`
  (bind _currenpath (`self.CurrenPath`))
  (bind _returnvalue (+ (`self.CurrentNodeIndex`) 1))
  (bind _exitpath (`/Game/Blueprints/WorldMapBPs/DungeonNodePath.ExitPath` _currenpath))
  (bind _exitnodeindex (`/Game/Blueprints/WorldMapBPs/DungeonNodePath.ExitNodeIndex` _currenpath))
  (bind _item (`KismetArrayLibrary.Array_Get` (`/Game/Blueprints/WorldMapBPs/DungeonNodePath.Nodes` (`self.CurrenPath`)) _returnvalue))
  (if (not (`self.Moving`))
    (`/Engine/EditorBlueprintResources/StandardMacros.IsValid` _item
      (:`Is Valid`
        (set `self.TargetNode` _item)
        (set `self.CurrentNodeIndex` _returnvalue))
      (:`Is Not Valid`
        (`/Engine/EditorBlueprintResources/StandardMacros.IsValid` _exitpath
          (:`Is Valid`
            (`self.UpdateNodeInfo` (`KismetArrayLibrary.Array_Get` (`/Game/Blueprints/WorldMapBPs/DungeonNodePath.Nodes` _exitpath) _exitnodeindex) _exitnodeindex)))))
    (`self.MoveToNode`)))

(fn `MoveToPreviousNode`
  (bind _currenpath (`self.CurrenPath`))
  (bind _returnvalue (+ (`self.CurrentNodeIndex`) -1))
  (bind _parentpath (`/Game/Blueprints/WorldMapBPs/DungeonNodePath.ParentPath` (`self.CurrenPath`)))
  (bind _parentnodeindex (`/Game/Blueprints/WorldMapBPs/DungeonNodePath.ParentNodeIndex` _currenpath))
  (bind _item (`KismetArrayLibrary.Array_Get` (`/Game/Blueprints/WorldMapBPs/DungeonNodePath.Nodes` _currenpath) _returnvalue))
  (if (not (`self.Moving`))
    (if (and (== (`self.CurrentNodeIndex`) 0) (`KismetSystemLibrary.IsValid` _parentpath))
      (`self.UpdateNodeInfo` (`KismetArrayLibrary.Array_Get` (`/Game/Blueprints/WorldMapBPs/DungeonNodePath.Nodes` _parentpath) _parentnodeindex) _parentnodeindex)
      (else
        (`/Engine/EditorBlueprintResources/StandardMacros.IsValid` _item
          (:`Is Valid`
            (`self.UpdateNodeInfo` _item _returnvalue)))))
    (`self.MoveToNode`)))

(fn `MoveToRightNode`
  (bind _currentnodeindex (`self.CurrentNodeIndex`))
  (if (not (`self.Moving`))
    (bind _childpath (`/Game/Blueprints/WorldMapBPs/DungeonNodePath.GetRightPathOfNode` (`self.MainPath`) _currentnodeindex))
    (`/Engine/EditorBlueprintResources/StandardMacros.IsValid` _childpath
      (:`Is Valid`
        (set `self.CurrenPath` _childpath)
        (if (== (`/Game/Blueprints/WorldMapBPs/DungeonNodePath.ExitNodeIndex` _childpath) _currentnodeindex)
          (bind _nodes (`/Game/Blueprints/WorldMapBPs/DungeonNodePath.Nodes` _childpath))
          (bind _returnvalue (- (`KismetArrayLibrary.Array_Length` (`/Game/Blueprints/WorldMapBPs/DungeonNodePath.Nodes` _childpath)) 1))
          (`self.UpdateNodeInfo` (`KismetArrayLibrary.Array_Get` _nodes _returnvalue) _returnvalue)
          (`self.MoveToNode` :!label _label)
          (elif (== (`/Game/Blueprints/WorldMapBPs/DungeonNodePath.ParentNodeIndex` _childpath) _currentnodeindex)
            (`self.UpdateNodeInfo` (`KismetArrayLibrary.Array_Get` _nodes))
            (goto _label)))))))

(fn `UpdateNodeInfo`
  (params (Target :type "/Game/Blueprints/WorldMapBPs/OLD_DungeonNode Object Reference") (Index :type Integer))
  (set `self.PreviousNode` (`self.CurrentNode`))
  (set `self.TargetNode` Target)
  (set `self.CurrentNodeIndex` Index))

(fn `UserConstructionScript`)