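; World map path actor that lays a mesh along a spline as a chain of spline mesh components.
; MakePath stores the given spacing and adds one segment per interval, using world-space spline positions and scaled directions as tangents on manually attached components.
; Each segment gets the configured mesh, material, collision mode and forward axis.
; The Construction Script does nothing; a duplicate of the build loop sits there disconnected, so paths build only when MakePath is called.
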(fn `MakePath`
  (params (InSpacing :type "Float (double-precision)"))
  (bind _tangentscale (`self.TangentScale`))
  (bind _spline (`self.Spline`))
  (bind _spacing (`self.Spacing`))
  (set `self.Spacing` InSpacing)
  (for _index (range (+ (`.ReturnValue` (`KismetMathLibrary.FMod` (`SplineComponent.GetSplineLength` _spline) _spacing)) 1))
    (bind _returnvalue (`AddComponent|SplineMeshComponent_1582` :`bManualAttachment` true))
    (bind _returnvalue_2 (* _index _spacing))
    (bind _returnvalue_3 (+ _returnvalue_2 _spacing))
    (`SplineMeshComponent.SetStartAndEnd` _returnvalue (`SplineComponent.GetWorldLocationAtDistanceAlongSpline` _spline _returnvalue_2) (* (`SplineComponent.GetWorldDirectionAtDistanceAlongSpline` _spline _returnvalue_2) _tangentscale) (`SplineComponent.GetWorldLocationAtDistanceAlongSpline` _spline _returnvalue_3) (* (`SplineComponent.GetWorldDirectionAtDistanceAlongSpline` _spline _returnvalue_3) _tangentscale))
    (`StaticMeshComponent.SetStaticMesh` _returnvalue (`self.SplineMesh`))
    (`PrimitiveComponent.SetMaterial` _returnvalue 0 (`self.SplineMaterial`))
    (switch `/Game/Blueprints/WorldMapBPs/WorldMapEnums/SplineCollisionEnum` (`self.CollisionEnum`)
      (:`NewEnumerator0`
        (`PrimitiveComponent.SetCollisionEnabled` _returnvalue "NoCollision"))
      (:`NewEnumerator1`
        (`PrimitiveComponent.SetCollisionEnabled` _returnvalue "QueryOnly"))
      (:`NewEnumerator2`
        (`PrimitiveComponent.SetCollisionEnabled` _returnvalue "QueryAndPhysics")))
    (switch `/Game/Blueprints/WorldMapBPs/WorldMapEnums/SplinePathForwardAxis` (`self.ForwardAxis`)
      (:`NewEnumerator0`
        (`SplineMeshComponent.SetForwardAxis` _returnvalue "X"))
      (:`NewEnumerator1`
        (`SplineMeshComponent.SetForwardAxis` _returnvalue "Y"))
      (:`NewEnumerator2`
        (`SplineMeshComponent.SetForwardAxis` _returnvalue "Z")))))

(fn `UserConstructionScript`)